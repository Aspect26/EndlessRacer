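; Coin multiplier pickup that temporarily boosts the coin multiplier when a vehicle drives into its Torus.
; On overlap with a VehicleBlueprint, it calls DoubleCoinMultiplier on the RunGameMode and hides itself, with the hidden flag blocking repeat triggers.
; The hidden actor stays alive as the timer, calling HalfCoinMultiplier after a fixed delay and then destroying itself.
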(event `self.Torus.OnComponentBeginOverlap`
  (params (OverlappedComponent :type "PrimitiveComponent Object Reference") (OtherActor :type "Actor Object Reference") (OtherComp :type "PrimitiveComponent Object Reference") (OtherBodyIndex :type Integer) (bFromSweep :type Boolean) (SweepResult :type "HitResult Structure (by ref)"))
  (if (not (`self.bHidden`))
    (cast `/Game/VehicleAdvBP/Blueprints/VehicleBlueprint` OtherActor)
    (bind _asrun_game_mode (cast `/Game/VehicleAdvBP/Blueprints/RunGameMode` (`GameplayStatics.GetGameMode`)))
    (`/Game/VehicleAdvBP/Blueprints/RunGameMode.Double Coin Multiplier` _asrun_game_mode)
    (`self.SetActorHiddenInGame` self true)
    (`KismetSystemLibrary.Delay` 25.0)
    (bind _asrun_game_mode_2 (cast `/Game/VehicleAdvBP/Blueprints/RunGameMode` (`GameplayStatics.GetGameMode`)))
    (`/Game/VehicleAdvBP/Blueprints/RunGameMode.Half Coin Multiplier` _asrun_game_mode_2)
    (`self.K2_DestroyActor`)))

(fn `UserConstructionScript`)