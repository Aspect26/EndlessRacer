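; FloorTileThinLeft is a floor tile Blueprint in the VehicleAdvBP game that supplies randomized coin spawn locations.
; GetCoinSpawnLocation inserts its coin spawn points into SpawnLocations, then returns a random selection from GetRandomLocationsFromArray at a 50 percent choice probability.
; The fourth insert has no named input, leaving CoinsSpawnLocation4 unused.
; The event graph is inactive, and the construction script only calls its parent.
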(fn `Get Coin Spawn Location`
  (returns (`Coins Location Box` :type "Array of BoxComponent Object Reference"))
  (locals (`Spawn Locations` :type "Array of BoxComponent Object Reference"))
  (`KismetArrayLibrary.Array_Insert` (`local.Spawn Locations`) (`self.CoinsSpawnLocation1`))
  (`KismetArrayLibrary.Array_Insert` (`local.Spawn Locations`) (`self.CoinsSpawnLocation2`))
  (`KismetArrayLibrary.Array_Insert` (`local.Spawn Locations`) (`self.CoinsSpawnLocation3`))
  (`KismetArrayLibrary.Array_Insert` (`local.Spawn Locations`))
  (`KismetArrayLibrary.Array_Insert` (`local.Spawn Locations`) (`self.CoinsSpawnLocation5`))
  (`KismetArrayLibrary.Array_Insert` (`local.Spawn Locations`) (`self.CoinsSpawnLocation6`))
  (bind _selected_box_collisions (`self.Get Random Locations From Array` (`local.Spawn Locations`)))
  (return _selected_box_collisions))

(fn `UserConstructionScript`
  (`parent.UserConstructionScript`))