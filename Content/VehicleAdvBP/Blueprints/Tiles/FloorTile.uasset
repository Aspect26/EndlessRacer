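; FloorTile is a floor segment for a runner mode that randomly populates itself with coins and power-ups.
; Its construction script randomly picks among two box areas, scatters coin child actors inside each pick, and sometimes adds a power-up.
; Overlapping EndCollision sets the RunGameMode checkpoint, requests another tile, then destroys this one after a long delay.
; GetAttachTransform exposes the AttachPoint transform.
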(event `self.EndCollision.OnComponentBeginOverlap`
  (params (OverlappedComponent :type "PrimitiveComponent Object Reference") (OtherActor :type "Actor Object Reference") (OtherComp :type "PrimitiveComponent Object Reference") (OtherBodyIndex :type Integer) (bFromSweep :type Boolean) (SweepResult :type "HitResult Structure (by ref)"))
  (bind _asrun_game_mode (cast `/Game/VehicleAdvBP/Blueprints/RunGameMode` (`GameplayStatics.GetGameMode`)))
  (`/Game/VehicleAdvBP/Blueprints/RunGameMode.Set Checkpoint` _asrun_game_mode (`SceneComponent.K2_GetComponentLocation` (`self.Checkpoint`)))
  (`/Game/VehicleAdvBP/Blueprints/RunGameMode.Add Floor Tile` _asrun_game_mode)
  (`KismetSystemLibrary.Delay` 120.0)
  (`self.K2_DestroyActor`))

(fn `Get Attach Transform`
  (returns (AttachPoint :type "Transform Structure"))
  (return (`SceneComponent.K2_GetComponentToWorld` (`self.AttachPoint`))))

(fn `Get Coin Spawn Location`
  (returns (`Coins Location Box` :type "Array of BoxComponent Object Reference"))
  (locals (`Spawn Locations` :type "Array of BoxComponent Object Reference"))
  (bind _spawn_locations (`local.Spawn Locations`))
  (`KismetArrayLibrary.Array_Insert` _spawn_locations (`self.CoinsSpawnLocation1`))
  (`KismetArrayLibrary.Array_Insert` _spawn_locations (`self.CoinsSpawnLocation2`))
  (bind _selected_box_collisions (`self.Get Random Locations From Array` _spawn_locations))
  (return _selected_box_collisions))

(fn `Get Random Locations From Array`
  (params (`Input Array` :type "Array of BoxComponent Object Reference") (`Choose Item Probability` :type Integer :default 50))
  (returns (`Selected Box Collisions` :type "Array of BoxComponent Object Reference"))
  (locals (`Selected Box Collicasions` :type "Array of BoxComponent Object Reference"))
  (bind _selected_box_collicasions (`local.Selected Box Collicasions`))
  (for _array_element `Input Array`
    (if (< (`KismetMathLibrary.RandomInteger` 100) `Choose Item Probability`)
      (`KismetArrayLibrary.Array_Insert` _selected_box_collicasions _array_element)))
  (return _selected_box_collicasions))

(fn `Spawn Coins Randomly`
  (locals (`Selected Coins Spawn Location` :type "BoxComponent Object Reference"))
  (bind _coins_location_box (`self.Get Coin Spawn Location` self))
  (for _array_element _coins_location_box
    (bind _output_get (set `self.Spawn Location Box` _array_element))
    (for _ (range 10)
      (`AddComponent|NODE_AddChildActorComponent-2` :`RelativeTransform` (`KismetMathLibrary.Conv_VectorToTransform` (`KismetMathLibrary.RandomPointInBoundingBox` (`SceneComponent.RelativeLocation` _output_get) (`BoxComponent.BoxExtent` _output_get)))))))

(fn `Spawn Power Up Randomly`
  (if (<= (`KismetMathLibrary.RandomInteger` 100) 33)
    (`AddComponent|NODE_AddChildActorComponent-3` :`RelativeTransform` (`KismetMathLibrary.Conv_VectorToTransform` (`SceneComponent.RelativeLocation` (`self.PowerUpSpawnLocation`))))))

(fn `UserConstructionScript`
  (locals (SelectedCoinsSpawnLocation :type "BoxComponent Object Reference"))
  (`|ExecutionSequence`
    (:`then_0`
      (`self.Spawn Coins Randomly`))
    (:`then_1`
      (`self.Spawn Power Up Randomly`))))