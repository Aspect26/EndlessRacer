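; Game mode for a vehicle runner that manages track generation, coins, checkpoints and respawning.
; AddFloorTile spawns a random tile class at the stored attach transform, then takes the next one from the new tile, chaining the track.
; Coin pickups scale by a multiplier that can be doubled or halved, and checkpoints only advance along X.
; RespawnVehicle spawns and possesses a vehicle at the checkpoint, passes on the camera setting and deducts coins, clamped at zero.
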(event `self.ReceiveBeginPlay`)

(event `Respawn Vehicle`
  (params (InCarCamera :type Boolean))
  (bind _returnvalue (`|SpawnActorFromClass` "/Game/VehicleAdvBP/Blueprints/VehicleBlueprint.VehicleBlueprint_C" (`KismetMathLibrary.Conv_VectorToTransform` (`self.Checkpoint`)) "AdjustIfPossibleButAlwaysSpawn" "OverrideRootScale" null null))
  (bind _output_get (set `self.NewVehicle` _returnvalue))
  (`/Game/VehicleAdvBP/Blueprints/VehicleBlueprint.SetCamera` _output_get InCarCamera)
  (`Controller.Possess` (`GameplayStatics.GetPlayerController` 0) _output_get)
  (`self.Apply Restart` self))

(fn `Add Coin`
  (set `self.Coins` (+ (`self.Coins`) (* 1 (`self.Coin Multiplier`)))))

(fn `Add Floor Tile`
  (bind _floortiles (`self.FloorTiles`))
  (bind _returnvalue (`|SpawnActorFromClass` (`|GetArrayItem` _floortiles (`KismetMathLibrary.RandomInteger` (`KismetArrayLibrary.Array_Length` _floortiles))) (`self.NextAtachPoint`) "Undefined" "OverrideRootScale" null null))
  (bind _asfloor_tile (cast `/Game/VehicleAdvBP/Blueprints/Tiles/FloorTile` _returnvalue))
  (bind _attachpoint (`/Game/VehicleAdvBP/Blueprints/Tiles/FloorTile.Get Attach Transform` _asfloor_tile))
  (set `self.NextAtachPoint` _attachpoint))

(fn `Apply Restart`
  ;[1 1 1] Decrease coins
  (bind _output_get (set `self.Coins` (- (`self.Coins`) 200)))
  (if (< _output_get 0)
    (set `self.Coins` 0)))

(fn `Double Coin Multiplier`
  (set `self.Coin Multiplier` (* (`self.Coin Multiplier`) 2)))

(fn `Get Checkpoint`
  (returns (Checkpoint :type "Vector Structure"))
  (return (`self.Checkpoint`)))

(fn `Get Coins Count`
  (returns (coins :type Integer))
  (return (`self.Coins`)))

(fn `Half Coin Multiplier`
  (set `self.Coin Multiplier` (/ (`self.Coin Multiplier`) 2)))

(fn `Set Checkpoint`
  (params (`Checkpoint Location` :type "Vector Structure"))
  (if (> (.x `Checkpoint Location`) (.x (`self.Checkpoint`)))
    (set `self.Checkpoint` `Checkpoint Location`)))

(fn `UserConstructionScript`)